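; BP_Grave is a graveyard grave whose soul can be reaped over a timed duration.
; ReapSoul subtracts the caller's DeltaTime from ReapTime until it hits zero, then marks the grave Reaped and returns completion and can-reap flags.
; Tick resets ReapTime to DefaultReapTime whenever IsBeingReaped is false, so an interrupted reap loses its progress.
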(event `self.ReceiveTick`
  (params (DeltaSeconds :type "Float (single-precision)"))
  (if (not (`self.IsBeingReaped`))
    (set `self.ReapTime` (`self.DefaultReapTime`))))

(fn `ReapSoul`
  (params (DeltaTime :type "Float (double-precision)"))
  (returns (FinishedReaping :type Boolean) (CanReap :type Boolean))
  (bind _reaped (`self.Reaped`))
  (if (not (`self.Reaped`))
    (set `self.ReapTime` (- (`self.ReapTime`) DeltaTime))
    (if (<= (`self.ReapTime`) 0.0)
      (`KismetSystemLibrary.PrintString` "Finished Reaping")
      (bind _output_get (set `self.Reaped` true))
      (return _output_get true)
      (else
        _)))
  (return _reaped (not _reaped)))

(fn `UserConstructionScript`)