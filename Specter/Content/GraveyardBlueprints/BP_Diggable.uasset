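; BP_Diggable is a gravestone that can be reaped over time to yield a randomly sized gold drop, set on BeginPlay.
; ReapTreasure counts ReapTime down by the passed delta, then spawns a BP_Gold above the GraveStone with that amount and marks it Reaped.
; Tick resets the timer whenever IsBeingReaped is false, so interrupted progress is lost, and disables Trigger collision once reaped.
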(event `self.ReceiveBeginPlay`
  (set `self.GoldAmount` (`KismetMathLibrary.RandomIntegerInRange` 4 12)))

(event `self.ReceiveTick`
  (params (DeltaSeconds :type "Float (single-precision)"))
  (if (`self.Reaped`)
    (`PrimitiveComponent.SetCollisionEnabled` (`self.Trigger`) "NoCollision"))
  (if (not (`self.IsBeingReaped`))
    (set `self.ReapTime` (`self.DefaultReapTime`))))

(fn `ReapTreasure`
  (params (DeltaTime :type "Float (double-precision)"))
  (returns (FinishedReaping :type Boolean) (CanReap :type Boolean))
  (bind _reaped (`self.Reaped`))
  (if (not (`self.Reaped`))
    (set `self.ReapTime` (- (`self.ReapTime`) DeltaTime))
    (if (<= (`self.ReapTime`) 0.0)
      (`KismetSystemLibrary.PrintString` "Finished Reaping")
      (`self.SpawnGold`)
      (bind _output_get (set `self.Reaped` true))
      (return _output_get true)
      (else
        _)))
  (return _reaped (not _reaped)))

(fn `SpawnGold`
  (bind (_returnvalue_location _returnvalue_rotation _returnvalue_scale) (`KismetMathLibrary.BreakTransform` (`SceneComponent.K2_GetComponentToWorld` (`self.GraveStone`))))
  (bind _returnvalue (`|SpawnActorFromClass` "/Game/GraveyardBlueprints/BP_Gold.BP_Gold_C" (`KismetMathLibrary.MakeTransform` (+ _returnvalue_location (0.0 0.0 50.0)) _returnvalue_rotation _returnvalue_scale) "Undefined" "OverrideRootScale" null null))
  (set `/Game/GraveyardBlueprints/BP_Gold.GoldAmount` (`self.GoldAmount`) _returnvalue))

(fn `UserConstructionScript`)