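; Spline-driven fence actor that builds a run of fence panels and middle posts along an editable spline.
; The construction script divides the spline length by FenceLength and adds a spline mesh panel per step, offsetting its start by half the post length.
; Each step after the first also adds a post spline mesh around the joint.
; Tangents are clamped to piece length, and all pieces have query and physics collision.
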(fn `UserConstructionScript`
  (bind _spline (`self.Spline`))
  (bind _spline_2 (`self.Spline`))
  (for _index (range (+ (`KismetMathLibrary.FTrunc` (/ (`SplineComponent.GetSplineLength` (`self.Spline`)) (`self.FenceLength`))) 1))
    (bind _returnvalue (`AddComponent|NODE_AddSplineMeshComponent-0`))
    (`SplineMeshComponent.SetForwardAxis` _returnvalue "X" true)
    (bind _returnvalue_2 (+ (/ (`self.MidPostLength`) 2.0) (* _index (`self.FenceLength`))))
    (bind _returnvalue_3 (* (+ _index 1) (`self.FenceLength`)))
    (`SplineMeshComponent.SetStartAndEnd` _returnvalue (`SplineComponent.GetLocationAtDistanceAlongSpline` _spline_2 _returnvalue_2 "Local") (`KismetMathLibrary.ClampVectorSize` (`SplineComponent.GetTangentAtDistanceAlongSpline` _spline_2 _returnvalue_2 "Local") 0.0 (`self.FenceLength`)) (`SplineComponent.GetLocationAtDistanceAlongSpline` _spline_2 _returnvalue_3 "Local") (`KismetMathLibrary.ClampVectorSize` (`SplineComponent.GetTangentAtDistanceAlongSpline` _spline_2 _returnvalue_3 "Local") 0.0 (`self.FenceLength`)) true)
    (`PrimitiveComponent.SetCollisionEnabled` _returnvalue "QueryAndPhysics")
    (if (> _index 0)
      (bind _returnvalue_4 (`AddComponent|NODE_AddSplineMeshComponent-2`))
      (`SplineMeshComponent.SetForwardAxis` _returnvalue_4 "X" true)
      (bind _returnvalue_5 (- (* _index (`self.FenceLength`)) (/ (`self.MidPostLength`) 2.0)))
      (bind _returnvalue_6 (+ (`self.MidPostLength`) (* _index (`self.FenceLength`))))
      (`SplineMeshComponent.SetStartAndEnd` _returnvalue_4 (`SplineComponent.GetLocationAtDistanceAlongSpline` _spline _returnvalue_5 "Local") (`KismetMathLibrary.ClampVectorSize` (`SplineComponent.GetTangentAtDistanceAlongSpline` _spline _returnvalue_5 "Local") 0.0 (`self.MidPostLength`)) (`SplineComponent.GetLocationAtDistanceAlongSpline` _spline _returnvalue_6 "Local") (`KismetMathLibrary.ClampVectorSize` (`SplineComponent.GetTangentAtDistanceAlongSpline` _spline _returnvalue_6 "Local") 0.0 (`self.MidPostLength`)) true)
      (`PrimitiveComponent.SetCollisionEnabled` _returnvalue_4 "QueryAndPhysics"))))